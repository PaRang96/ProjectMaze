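; BP_DS_Spike is a short-lived spike hazard that damages the player on contact.
; A hit on the Spike component applies a small fixed amount of damage if the other actor is the player pawn, and destroys the spike whatever it hits.
; Tick accumulates elapsed time and destroys the actor after about two seconds if nothing has been hit.
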(event OnComponentHit(Spike)
  (params (HitComponent :type Primitive%20Component%20Object%20Reference) (OtherActor :type Actor%20Object%20Reference) (OtherComp :type Primitive%20Component%20Object%20Reference) (NormalImpulse :type Vector :default "0, 0, 0") (Hit :type Hit%20Result%20Structure%20%28by%20ref%29))
  (if (== OtherActor (Game|Player|GetPlayerPawn 0))
    (Game|Damage|ApplyDamage OtherActor 2.0 0 0)
    (Actor|DestroyActor)
    (else
      (Actor|DestroyActor))))

(event EventTick
  (params (DeltaSeconds :type Float%20%28single-precision%29))
  (bind _output_get (Variables|Default|SetTime (+ DeltaSeconds (Variables|Default|GetTime))))
  (if (> _output_get 2.0)
    (Actor|DestroyActor)))

(fn ConstructionScript)