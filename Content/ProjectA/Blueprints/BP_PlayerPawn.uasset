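; Player character that handles movement, look, health, a dash and interaction with tagged objects.
; Damage reduces HP, and reaching zero tells the in-game HUD to show death once.
; Dash launches the character along the mesh's right vector, gated by a Tick-driven timer that must equal Cooldown and resets on use.
; Capsule overlaps with "InteractionObject" components and the Interaction input fire event dispatchers for prompts and interaction.
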(event OnComponentBeginOverlap(CapsuleComponent)
  (params (OverlappedComponent :type Primitive%20Component%20Object%20Reference) (OtherActor :type Actor%20Object%20Reference) (OtherComp :type Primitive%20Component%20Object%20Reference) (OtherBodyIndex :type Integer) (bFromSweep :type Boolean) (SweepResult :type Hit%20Result%20Structure%20%28by%20ref%29))
  ;[1 1 1] Interaction Message
  (if (Components|ComponentHasTag OtherComp "InteractionObject")
    (Default|CallShowInteractionMessage)))

(event OnComponentEndOverlap(CapsuleComponent)
  (params (OverlappedComponent :type Primitive%20Component%20Object%20Reference) (OtherActor :type Actor%20Object%20Reference) (OtherComp :type Primitive%20Component%20Object%20Reference) (OtherBodyIndex :type Integer))
  ;[1 1 1] Interaction Message
  (if (Components|ComponentHasTag OtherComp "InteractionObject")
    (Default|CallDisableInteractionMessage)))

(event EventBeginPlay
  (Variables|Default|SetCurrentHP (Variables|Default|GetMaxHP)))

(event Game|Damage|EventAnyDamage
  (params (Damage :type Float%20%28single-precision%29) (DamageType :type Damage%20Type%20Object%20Reference) (InstigatedBy :type Controller%20Object%20Reference) (DamageCauser :type Actor%20Object%20Reference))
  ;[1 1 1] Damage Calculation & Death
  (bind _output_get (Variables|Default|SetCurrentHP (- (Variables|Default|GetCurrentHP) (Math|Float|Truncate Damage))))
  (if (<= _output_get 0)
    (Utilities|FlowControl|DoOnce false
      (:Completed
        (bind _asbp_in_game_hud (Utilities|Casting|CastToBP_InGameHUD (HUD|GetHUD (Game|GetPlayerController 0))))
        (Default|SetDie _asbp_in_game_hud)))))

(event EventTick
  (params (DeltaSeconds :type Float%20%28single-precision%29))
  ;[1 1 1] Dash Cooldown
  (bind _output_get (Variables|Default|SetCooldownRate (+ DeltaSeconds (Variables|Default|GetCooldownRate))))
  (if (>= _output_get 5.0)
    (Variables|Default|SetCooldownRate 5.0)))

(event Input|ActionEvents|InputActionInteraction
  (params (Key :type Key%20Structure :default "None"))
  ;[1 1 1] Actual Interaction
  (:Pressed
    (Default|CallInteractionDispatcher)))

(event Input|ActionEvents|InputActionDash
  (params (Key :type Key%20Structure :default "None"))
  ;[1 1 1] Dash
  (:Pressed
    (if (== (Variables|Default|GetCooldownRate) (Variables|Default|GetCooldown))
      (Utilities|FlowControl|DoOnce false :!label _label
        (:Completed
          (Character|LaunchCharacter (* (Math|Vector|GetRightVector (Variables|/Script/Engine.Character|GetMesh (Game|GetPlayerCharacter 0))) (Variables|Default|GetDashPower)) false false)
          (Variables|Default|SetCooldownRate 0.0)
          (goto _label Reset))))))

(event Input|AxisEvents|InputAxisTurn
  (params (AxisValue :type Float%20%28single-precision%29))
  ;[1 1 1] Character Rotation
  (Pawn|Input|AddControllerYawInput AxisValue))

(event Input|AxisEvents|InputAxisLookUp
  (params (AxisValue :type Float%20%28single-precision%29))
  ;[1 1 1] Character Rotation
  (Pawn|Input|AddControllerPitchInput AxisValue))

(event Input|AxisEvents|InputAxisMoveForward
  (params (AxisValue :type Float%20%28single-precision%29))
  ;[1 1 1] Character Movement
  (Pawn|Input|AddMovementInput (Math|Vector|GetForwardVector (Math|Rotator|MakeRotator 0.0 0.0 (.Yaw (Math|Rotator|BreakRotator (Pawn|GetControlRotation :!class /Script/Engine.Pawn))))) AxisValue false))

(event Input|AxisEvents|InputAxisMoveRight
  (params (AxisValue :type Float%20%28single-precision%29))
  ;[1 1 1] Character Movement
  (Pawn|Input|AddMovementInput (Math|Vector|GetRightVector (Math|Rotator|MakeRotator 0.0 0.0 (.Yaw (Math|Rotator|BreakRotator (Pawn|GetControlRotation :!class /Script/Engine.Pawn))))) AxisValue false))

(fn ConstructionScript)