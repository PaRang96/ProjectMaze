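; BP_SpikeSpawner is an actor that spawns BP_DS_Spike actors while the player pawn is within a set distance.
; Each Tick compares the distance to player pawn 0 against DistanceSetting.
; In range, a Delay throttles spawning at the Arrow component's transform to roughly every two seconds.
; A parallel Sequence branch calls PlaySoundAtLocation at the world origin on every in-range tick, with no sound asset shown.
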(event EventTick
  (params (DeltaSeconds :type Float%20%28single-precision%29))
  (bind _output_get (Variables|Default|SetActualDistance (Transformation|GetDistanceTo (Game|Player|GetPlayerPawn 0))))
  (if (<= _output_get (Variables|Default|GetDistanceSetting))
    (Utilities|FlowControl|Sequence
      (:then_0
        (Utilities|FlowControl|Delay 2.0)
        (Game|SpawnActorfromClass "/Game/ProjectA/Blueprints/BP_DS_Spike.BP_DS_Spike_C" (Transformation|GetWorldTransform (Variables|Default|GetArrow)) "Undefined" 0 0))
      (:then_1
        (Audio|PlaySoundatLocation 0 "0, 0, 0" "0, 0, 0" 1.0 1.0 0.0 0 0 0)))))

(fn ConstructionScript)