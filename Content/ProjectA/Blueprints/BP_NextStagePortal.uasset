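; BP_NextStagePortal is a portal that loads the next stage when the player interacts with it inside its trigger box.
; Box overlap begin and end bind and unbind an event on the BP_PlayerPawn interaction dispatcher.
; InteractionFunc opens the level named by the LevelName variable, then resets the player pawn's EnergyNum to zero.
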(event OnComponentBeginOverlap(Box)
  (params (OverlappedComponent :type Primitive%20Component%20Object%20Reference) (OtherActor :type Actor%20Object%20Reference) (OtherComp :type Primitive%20Component%20Object%20Reference) (OtherBodyIndex :type Integer) (bFromSweep :type Boolean) (SweepResult :type Hit%20Result%20Structure%20%28by%20ref%29))
  (bind _asbp_player_pawn (Utilities|Casting|CastToBP_PlayerPawn OtherActor))
  (EventDispatchers|BindEventtoInteractionDispatcher _asbp_player_pawn (EventDispatchers|CreateEvent :!event InteractionFunc)))

(event OnComponentEndOverlap(Box)
  (params (OverlappedComponent :type Primitive%20Component%20Object%20Reference) (OtherActor :type Actor%20Object%20Reference) (OtherComp :type Primitive%20Component%20Object%20Reference) (OtherBodyIndex :type Integer))
  (bind _asbp_player_pawn (Utilities|Casting|CastToBP_PlayerPawn OtherActor))
  (EventDispatchers|UnbindEventfromInteractionDispatcher _asbp_player_pawn (EventDispatchers|CreateEvent :!event InteractionFunc)))

(fn ConstructionScript)

(fn InteractionFunc
  (Game|OpenLevel(byName) (Variables|Default|GetLevel%20Name))
  (bind _asbp_player_pawn (Utilities|Casting|CastToBP_PlayerPawn (Game|Player|GetPlayerPawn 0)))
  (Variables|/Game/ProjectA/Blueprints/BP_PlayerPawn.BP_PlayerPawn_C|SetEnergyNum _asbp_player_pawn 0))