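; Torch actor whose point light turns on while the first player's pawn is within a set distance.
; Each tick it checks that distance and plays a timeline that drives the light intensity.
; Out of range, it sets the intensity to zero and stops the timeline.
; The in-range branch also calls a placeholder sound at the world origin every tick, with no sound assigned.
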(event EventTick
  (params (DeltaSeconds :type Float%20%28single-precision%29))
  (bind _output_get (Variables|Default|SetActualDistance (Transformation|GetDistanceTo (Game|Player|GetPlayerPawn 0))))
  (if (<= _output_get (Variables|Default|GetDistanceSetting))
    (Utilities|FlowControl|Sequence
      (:then_0
        ;[1 1 1] need sound
        (Audio|PlaySoundatLocation 0 "0, 0, 0" "0, 0, 0" 1.0 1.0 0.0 0 0 0))
      (:then_1
        (bind _newtrack_0 (Timeline|TorchIntensity Play)
          (:Update
            (Rendering|Components|Light|SetIntensity (Variables|Default|GetPointLight) (* _newtrack_0 1.5e+03))))))
    (else
      (Rendering|Components|Light|SetIntensity (Variables|Default|GetPointLight) 0.0)
      (Timeline|TorchIntensity Stop))))

(fn ConstructionScript)