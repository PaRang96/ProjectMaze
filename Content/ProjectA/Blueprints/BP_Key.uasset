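; BP_Key is a collectible key whose Skull component floats on a timeline that applies Z offsets from BeginPlay.
; Its Box overlap binds and unbinds an event on the BP_PlayerPawn interaction dispatcher, apparently KeyPickup, so pickup works only in range.
; KeyPickup increments the pawn's KeyNum, calls a placeholder sound at the world origin and destroys the key.
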(event OnComponentBeginOverlap(Box)
  (params (OverlappedComponent :type Primitive%20Component%20Object%20Reference) (OtherActor :type Actor%20Object%20Reference) (OtherComp :type Primitive%20Component%20Object%20Reference) (OtherBodyIndex :type Integer) (bFromSweep :type Boolean) (SweepResult :type Hit%20Result%20Structure%20%28by%20ref%29))
  (bind _asbp_player_pawn (Utilities|Casting|CastToBP_PlayerPawn OtherActor))
  (EventDispatchers|BindEventtoInteractionDispatcher _asbp_player_pawn (EventDispatchers|CreateEvent :!event KeyPickup)))

(event OnComponentEndOverlap(Box)
  (params (OverlappedComponent :type Primitive%20Component%20Object%20Reference) (OtherActor :type Actor%20Object%20Reference) (OtherComp :type Primitive%20Component%20Object%20Reference) (OtherBodyIndex :type Integer))
  (bind _asbp_player_pawn (Utilities|Casting|CastToBP_PlayerPawn OtherActor))
  (EventDispatchers|UnbindEventfromInteractionDispatcher _asbp_player_pawn (EventDispatchers|CreateEvent :!event KeyPickup)))

(event EventBeginPlay
  (bind _float (Timeline|KeyFloat Play)
    (:Update
      (Transformation|AddLocalOffset (Variables|Default|GetSkull) (Math|Vector|MakeVector 0.0 0.0 _float) false false))))

(fn ConstructionScript)

(fn KeyPickup
  (bind _returnvalue (Actor|GetActorOfClass "/Game/ProjectA/Blueprints/BP_PlayerPawn.BP_PlayerPawn_C"))
  (Math|Integer|IncrementInt (Variables|/Game/ProjectA/Blueprints/BP_PlayerPawn.BP_PlayerPawn_C|GetKeyNum _returnvalue)
    (:%20%20
      ;[1 1 1] need sound
      (Audio|PlaySoundatLocation 0 "0, 0, 0" "0, 0, 0" 1.0 1.0 0.0 0 0 0)
      (Actor|DestroyActor))))