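; BP_Door is a locked door that opens by sinking when the player has a key.
; Its box binds and unbinds an event on BP_PlayerPawn's interaction dispatcher as the pawn enters and leaves.
; DoorOpen spends a key, plays a sound, shakes the camera and starts a looping timer that lowers the door, or prints a no-key message.
; The below-zero height check for destroying the actor runs only inside DoorOpen, not on timer ticks.
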(event OnComponentBeginOverlap(Box)
  (params (OverlappedComponent :type Primitive%20Component%20Object%20Reference) (OtherActor :type Actor%20Object%20Reference) (OtherComp :type Primitive%20Component%20Object%20Reference) (OtherBodyIndex :type Integer) (bFromSweep :type Boolean) (SweepResult :type Hit%20Result%20Structure%20%28by%20ref%29))
  (bind _asbp_player_pawn (Utilities|Casting|CastToBP_PlayerPawn OtherActor))
  (EventDispatchers|BindEventtoInteractionDispatcher _asbp_player_pawn (EventDispatchers|CreateEvent :!event DoorOpen)))

(event OnComponentEndOverlap(Box)
  (params (OverlappedComponent :type Primitive%20Component%20Object%20Reference) (OtherActor :type Actor%20Object%20Reference) (OtherComp :type Primitive%20Component%20Object%20Reference) (OtherBodyIndex :type Integer))
  (bind _asbp_player_pawn (Utilities|Casting|CastToBP_PlayerPawn OtherActor))
  (EventDispatchers|UnbindEventfromInteractionDispatcher _asbp_player_pawn (EventDispatchers|CreateEvent :!event DoorOpen)))

(fn ConstructionScript)

(fn DoorOpen
  (bind _newparam (CallFunction|CheckKeynum))
  (if _newparam
    (Utilities|FlowControl|Sequence
      (:then_0
        (Audio|PlaySoundatLocation 0 (Transformation|GetWorldLocation (Variables|Default|GetDoor)) "0, 0, 0" 1.0 1.0 0.0 0 0 0))
      (:then_1
        (Utilities|Time|SetTimerbyFunctionName 0 "DoorOpenFunction" 0.01 true)
        (if (< (.z (Transformation|GetWorldLocation (Variables|Default|GetDoor))) 0.0)
          (Actor|DestroyActor)))
      (:then_2
        (CameraShakes|StartCameraShake (Game|GetPlayerCameraManager 0) "/Game/ProjectA/Blueprints/BP_CameraShaker.BP_CameraShaker_C" 1.0 "CameraLocal" "0, 0, 0")))
    (else
      (Development|PrintString "Currently has no key"))))

(fn CheckKeynum
  (bind _returnvalue (Actor|GetActorOfClass "/Game/ProjectA/Blueprints/BP_PlayerPawn.BP_PlayerPawn_C"))
  (if (>= (Variables|/Game/ProjectA/Blueprints/BP_PlayerPawn.BP_PlayerPawn_C|GetKeyNum _returnvalue) 1)
    (Math|Integer|DecrementInt (Variables|/Game/ProjectA/Blueprints/BP_PlayerPawn.BP_PlayerPawn_C|GetKeyNum _returnvalue)
      (:%20%20
        (return true)))
    (else
      (return false))))

(fn DoorOpenFunction
  (Transformation|AddWorldOffset (Variables|Default|GetDoor) (* (Math|Vector|GetUpVector (Transformation|GetWorldRotation (Variables|Default|GetDoor))) -3.0) false false))