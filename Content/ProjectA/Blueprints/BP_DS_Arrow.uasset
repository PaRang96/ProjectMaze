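; BP_DS_Arrow is a physics-driven arrow projectile that damages the player on contact.
; On BeginPlay it launches itself with an impulse along ArrowBody's up vector.
; On overlap it damages the player pawn if hit, then stops physics and collision and destroys itself after a brief delay.
; Non-player hits wait a moment before freezing and linger longer before being destroyed.
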(event OnComponentBeginOverlap(ArrowBody)
  (params (OverlappedComponent :type Primitive%20Component%20Object%20Reference) (OtherActor :type Actor%20Object%20Reference) (OtherComp :type Primitive%20Component%20Object%20Reference) (OtherBodyIndex :type Integer) (bFromSweep :type Boolean) (SweepResult :type Hit%20Result%20Structure%20%28by%20ref%29))
  (bind _arrowbody (Variables|Default|GetArrowBody))
  (bind _arrowbody_2 (Variables|Default|GetArrowBody))
  (if (== OtherActor (Game|Player|GetPlayerPawn 0))
    (Game|Damage|ApplyDamage OtherActor 1.0 0 0)
    (Physics|SetSimulatePhysics _arrowbody false)
    (Collision|SetCollisionEnabled _arrowbody "NoCollision")
    (Utilities|FlowControl|Delay 0.2)
    (Actor|DestroyActor)
    (else
      (Utilities|FlowControl|Delay 0.05)
      (Physics|SetSimulatePhysics _arrowbody_2 false)
      (Collision|SetCollisionEnabled _arrowbody_2 "NoCollision")
      (Utilities|FlowControl|Delay 0.8)
      (Actor|DestroyActor))))

(event EventBeginPlay
  (bind _arrowbody (Variables|Default|GetArrowBody))
  (Physics|AddImpulse _arrowbody (* (Math|Vector|GetUpVector _arrowbody) 3e+03) "None" false))

(fn ConstructionScript)