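; BP_AI is an AI-controlled enemy that hurts the player on contact, or is destroyed if the player's energy count is exactly five.
; On BeginPlay it spawns its default controller and initializes the BB_AI blackboard on it; no behavior tree is started here.
; Capsule hits against BP_PlayerPawn check EnergyNum to choose between destroying itself and applying fixed damage to the player.
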(event OnComponentHit(CapsuleComponent)
  (params (HitComponent :type Primitive%20Component%20Object%20Reference) (OtherActor :type Actor%20Object%20Reference) (OtherComp :type Primitive%20Component%20Object%20Reference) (NormalImpulse :type Vector :default "0, 0, 0") (Hit :type Hit%20Result%20Structure%20%28by%20ref%29))
  (bind _asbp_player_pawn (Utilities|Casting|CastToBP_PlayerPawn OtherActor))
  (if (== (Variables|/Game/ProjectA/Blueprints/BP_PlayerPawn.BP_PlayerPawn_C|GetEnergyNum _asbp_player_pawn) 5)
    (Actor|DestroyActor)
    (else
      (Game|Damage|ApplyDamage _asbp_player_pawn 5.0 0 0))))

(event EventTick
  (params (DeltaSeconds :type Float%20%28single-precision%29)))

(event EventBeginPlay
  (Pawn|SpawnDefaultController)
  (Class|AIController|UseBlackboard (AI|GetAIController (Pawn|GetController)) "/Game/ProjectA/AI/BB_AI.BB_AI"))

(fn ConstructionScript)